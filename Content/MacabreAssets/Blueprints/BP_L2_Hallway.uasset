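; BP_L2_Hallway is an interaction trigger that lets the player light the sub-basement sconces in a hallway.
; Overlapping L2_Collider enables input and, until LitTorches is set, shows a FlashlightHUD prompt that depends on holding inventory item "K2".
; Pressing the trigger action in range with that item messages every BP_SubBasement_Sconce to light, clears the prompt and consumes the item.
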(event OnComponentEndOverlap(L2_Collider)
  (params (OtherActor :type Actor%20Object%20Reference) (OtherComp :type Primitive%20Component%20Object%20Reference) (OtherBodyIndex :type Integer))
  (Variables|Default|SetInRange false)
  (bind _outactors (Actor|GetAllActorsOfClass "/Game/MacabreAssets/Blueprints/FlashlightHUD.FlashlightHUD_C"))
  (Class|HUDInterface|ClearCurrentMessage(Message) (Utilities|Array|Get(acopy) _outactors)))

(event OnComponentBeginOverlap(L2_Collider)
  (params (OtherActor :type Actor%20Object%20Reference) (OtherComp :type Primitive%20Component%20Object%20Reference) (OtherBodyIndex :type Integer) (bFromSweep :type Boolean) (SweepResult :type Hit%20Result%20Structure%20%28by%20ref%29))
  (Variables|Default|SetInRange true)
  (Input|EnableInput (Game|GetPlayerController 0))
  (if (not (Variables|Default|GetLitTorches))
    (bind _outactors (Actor|GetAllActorsOfClass "/Game/MacabreAssets/Blueprints/FlashlightHUD.FlashlightHUD_C"))
    (bind _hasitem (Class|InventoryInterface|CheckInventory(Message) OtherActor "K2"))
    (if _hasitem
      (Class|HUDInterface|DisplayMessage(Message) (Utilities|Array|Get(acopy) _outactors) "Press 'E' or (X) to light sconces")
      (else
        (Class|HUDInterface|DisplayMessage(Message) (Utilities|Array|Get(acopy) _outactors) "I need to find a torch to light these sconces...")))))

(event EventBeginPlay)

(event EventActorBeginOverlap
  (params (OtherActor :type Actor%20Object%20Reference)))

(event EventTick
  (params (DeltaSeconds :type Float%20%28single-precision%29)))

(event Input|ActionEvents|InputActionEventTrigger
  (:Pressed
    (if (Variables|Default|GetInRange)
      (bind _hasitem (Class|InventoryInterface|CheckInventory(Message) (stale OnComponentBeginOverlap(L2_Collider) OtherActor) "K2"))
      (if _hasitem
        (bind _outactors (Actor|GetAllActorsOfClass "/Game/MacabreAssets/Blueprints/BP_SubBasement_Sconce.BP_SubBasement_Sconce_C"))
        (for _array_element _outactors
          (Class|LightInterface|LightSconces(Message) _array_element))
        (bind _outactors_2 (Actor|GetAllActorsOfClass "/Game/MacabreAssets/Blueprints/FlashlightHUD.FlashlightHUD_C"))
        (Class|HUDInterface|ClearCurrentMessage(Message) (Utilities|Array|Get(acopy) _outactors_2))
        (Variables|Default|SetLitTorches true)
        (Class|InventoryInterface|RemoveInventory(Message) (Game|GetPlayerCharacter 0) "K2")))))

(fn ConstructionScript)