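; BP_K3_Orb is a pickup orb that adds the "K3" item to inventory and triggers door slams.
; Box overlap enables input and shows a prompt through FlashlightHUD, which clears when the overlap ends.
; Pressing Event Trigger in range messages the overlapping actor to add the item, destroys a component and sets PickedUp.
; The pickup then sends a slam message to every BP_Slammable_Door in the level.
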(event OnComponentBeginOverlap(Box)
  (params (OtherActor :type Actor%20Object%20Reference) (OtherComp :type Primitive%20Component%20Object%20Reference) (OtherBodyIndex :type Integer) (bFromSweep :type Boolean) (SweepResult :type Hit%20Result%20Structure%20%28by%20ref%29))
  (if (not (Variables|Default|GetPickedUp))
    (Variables|Default|SetInRange true)
    (Input|EnableInput (Game|GetPlayerController 0))
    (bind _outactors (Actor|GetAllActorsOfClass "/Game/MacabreAssets/Blueprints/FlashlightHUD.FlashlightHUD_C"))
    (Class|HUDInterface|DisplayMessage(Message) (Utilities|Array|Get(acopy) _outactors) "Press 'E' or (X) to pick up orb")))

(event OnComponentEndOverlap(Box)
  (params (OtherActor :type Actor%20Object%20Reference) (OtherComp :type Primitive%20Component%20Object%20Reference) (OtherBodyIndex :type Integer))
  (Variables|Default|SetInRange false)
  (bind _outactors (Actor|GetAllActorsOfClass "/Game/MacabreAssets/Blueprints/FlashlightHUD.FlashlightHUD_C"))
  (Class|HUDInterface|ClearCurrentMessage(Message) (Utilities|Array|Get(acopy) _outactors)))

(event Input|ActionEvents|InputActionEventTrigger
  (:Pressed
    (if (Variables|Default|GetInRange)
      (Class|InventoryInterface|AddInventory(Message) (stale OnComponentBeginOverlap(Box) OtherActor) "K3")
      (Components|DestroyComponent)
      (bind _outactors (Actor|GetAllActorsOfClass "/Game/MacabreAssets/Blueprints/FlashlightHUD.FlashlightHUD_C"))
      (Class|HUDInterface|ClearCurrentMessage(Message) (Utilities|Array|Get(acopy) _outactors))
      (Variables|Default|SetPickedUp true)
      (bind _outactors_2 (Actor|GetAllActorsOfClass "/Game/MacabreAssets/Blueprints/BP_Slammable_Door.BP_Slammable_Door_C"))
      (for _array_element _outactors_2
        (Class|EventManager|SlamDoor(Message) _array_element)))))

(fn ConstructionScript)