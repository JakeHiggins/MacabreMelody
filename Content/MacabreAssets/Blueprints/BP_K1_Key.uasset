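; BP_K1_Key is a pickup key that the player collects with E while inside its collision volume.
; Overlap sets an in-range flag, enables player input and shows a prompt on the FlashlightHUD; leaving clears both flag and prompt.
; Pressing E in range passes "K1" to the overlapping actor's AddInventoryMessage, destroys the key and clears the HUD message.
; Overlap does not filter by actor type, and input is never disabled on exit.
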(event OnComponentEndOverlap(PickupCollision)
  (params (OtherActor :type Actor%20Object%20Reference) (OtherComp :type Primitive%20Component%20Object%20Reference) (OtherBodyIndex :type Integer))
  (Variables|Default|SetInRange false)
  (bind _outactors (Actor|GetAllActorsOfClass "/Game/MacabreAssets/Blueprints/FlashlightHUD.FlashlightHUD_C"))
  (Default|ClearCurrentMessage (Utilities|Array|Get(acopy) _outactors)))

(event OnComponentBeginOverlap(PickupCollision)
  (params (OtherActor :type Actor%20Object%20Reference) (OtherComp :type Primitive%20Component%20Object%20Reference) (OtherBodyIndex :type Integer) (bFromSweep :type Boolean) (SweepResult :type Hit%20Result%20Structure%20%28by%20ref%29))
  (if (not (Variables|Default|GetPickedUp))
    (Variables|Default|SetInRange true)
    (Input|EnableInput (Game|GetPlayerController 0))
    (bind _outactors (Actor|GetAllActorsOfClass "/Game/MacabreAssets/Blueprints/FlashlightHUD.FlashlightHUD_C"))
    (Default|DisplayMessage (Utilities|Array|Get(acopy) _outactors) "\"Press 'E' to pick up key")))

(event EventBeginPlay)

(event EventActorBeginOverlap
  (params (OtherActor :type Actor%20Object%20Reference)))

(event EventTick
  (params (DeltaSeconds :type Float%20%28single-precision%29)))

(event Input|KeyboardEvents|E
  (:Pressed
    (if (Variables|Default|GetInRange)
      (Class|InventoryInterface|AddInventory(Message) (stale OnComponentBeginOverlap(PickupCollision) OtherActor) "K1")
      (Actor|DestroyActor)
      (bind _outactors (Actor|GetAllActorsOfClass "/Game/MacabreAssets/Blueprints/FlashlightHUD.FlashlightHUD_C"))
      (Default|ClearCurrentMessage (Utilities|Array|Get(acopy) _outactors))
      (Variables|Default|SetPickedUp true))))

(fn ConstructionScript)