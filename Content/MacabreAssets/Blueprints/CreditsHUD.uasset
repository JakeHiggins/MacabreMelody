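; HUD Blueprint that draws the game's credits screen in white text.
; DrawHUD renders the title, creator line, audio credits list and closing thanks through individual DrawText calls, with text held in variables.
; The title and thanks are offset from the horizontal center near the top and bottom, while the audio block stacks downward from AudioX and AudioY variables.
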(event EventDrawHUD
  (params (SizeX :type Integer) (SizeY :type Integer))
  ;[1 1 1] Draw Title
  (HUD|DrawText (Variables|Default|GetTitle) "(R=1.000000,G=1.000000,B=1.000000,A=1.000000)" (Math|Conversions|ToFloat(Integer) (- (/ SizeX 2) 100)) (Math|Conversions|ToFloat(Integer) (- 50 0)) 0 2.0 false)
  (HUD|DrawText (Variables|Default|GetCreated%20By) "(R=1.000000,G=1.000000,B=1.000000,A=1.000000)" (Math|Conversions|ToFloat(Integer) (- (/ SizeX 2) 95)) (Variables|Default|GetCreatedY) 0 1.25 false)
  (HUD|DrawText (Variables|Default|GetAudio%20Credits) "(R=1.000000,G=1.000000,B=1.000000,A=1.000000)" (Variables|Default|GetAudioX) (Variables|Default|GetAudioY) 0 1.25 false)
  (HUD|DrawText (Variables|Default|GetBackgroundMusic) "(R=1.000000,G=1.000000,B=1.000000,A=1.000000)" (Variables|Default|GetAudioX) (+ (Variables|Default|GetAudioY) 4e+01) 0 1.0 false)
  (HUD|DrawText (Variables|Default|GetMiller) "(R=1.000000,G=1.000000,B=1.000000,A=1.000000)" (Variables|Default|GetAudioX) (+ (Variables|Default|GetAudioY) 7e+01) 0 1.0 false)
  (HUD|DrawText (Variables|Default|GetPalumbo) "(R=1.000000,G=1.000000,B=1.000000,A=1.000000)" (Variables|Default|GetAudioX) (+ (Variables|Default|GetAudioY) 1e+02) 0 1.0 false)
  (HUD|DrawText (Variables|Default|GetDavid) "(R=1.000000,G=1.000000,B=1.000000,A=1.000000)" (Variables|Default|GetAudioX) (+ (Variables|Default|GetAudioY) 1.3e+02) 0 1.0 false)
  (HUD|DrawText (Variables|Default|GetDonny%20) "(R=1.000000,G=1.000000,B=1.000000,A=1.000000)" (Variables|Default|GetAudioX) (+ (Variables|Default|GetAudioY) 1.6e+02) 0 1.0 false)
  (HUD|DrawText (Variables|Default|GetLocket) "(R=1.000000,G=1.000000,B=1.000000,A=1.000000)" (Variables|Default|GetAudioX) (+ (Variables|Default|GetAudioY) 1.9e+02) 0 1.0 false)
  (HUD|DrawText (Variables|Default|GetThanks) "(R=1.000000,G=1.000000,B=1.000000,A=1.000000)" (Math|Conversions|ToFloat(Integer) (- (/ SizeX 2) 125)) (Math|Conversions|ToFloat(Integer) (- SizeY 100)) 0 2.0 false))

(fn ConstructionScript)