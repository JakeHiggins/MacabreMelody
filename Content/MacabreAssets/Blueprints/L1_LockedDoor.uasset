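; Level 1 locked double door that the player unlocks with inventory key "K1" by pressing E near its collider.
; Overlap enables input and shows a FlashlightHUD prompt; a successful key check clears it and removes the key.
; Tick plays a timeline while Opening, adding speed offsets to both leaves' relative locations each update.
; End overlap clears the prompt but sets InRange true, so E stays active after leaving.
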(event OnComponentEndOverlap(L1_Collider)
  (params (OtherActor :type Actor%20Object%20Reference) (OtherComp :type Primitive%20Component%20Object%20Reference) (OtherBodyIndex :type Integer))
  (Variables|Default|SetInRange true)
  (bind _outactors (Actor|GetAllActorsOfClass "/Game/MacabreAssets/Blueprints/FlashlightHUD.FlashlightHUD_C"))
  (Class|HUDInterface|ClearCurrentMessage(Message) (Utilities|Array|Get(acopy) _outactors)))

(event OnComponentBeginOverlap(L1_Collider)
  (params (OtherActor :type Actor%20Object%20Reference) (OtherComp :type Primitive%20Component%20Object%20Reference) (OtherBodyIndex :type Integer) (bFromSweep :type Boolean) (SweepResult :type Hit%20Result%20Structure%20%28by%20ref%29))
  (Variables|Default|SetInRange true)
  (Input|EnableInput (Game|GetPlayerController 0))
  (if (not (Variables|Default|GetIsOpen))
    (bind _outactors (Actor|GetAllActorsOfClass "/Game/MacabreAssets/Blueprints/FlashlightHUD.FlashlightHUD_C"))
    (Class|HUDInterface|DisplayMessage(Message) (Utilities|Array|Get(acopy) _outactors) "Press 'E' to unlock door")))

(event EventTick
  (params (DeltaSeconds :type Float%20%28single-precision%29))
  (if (Variables|Default|GetOpening)
    (bind (_direction _leftspeed _rightspeed) (Timeline|OpenDoorAnim Play)
      (:Update
        (Transformation|SetRelativeLocation (+ _leftspeed (Variables|/Script/Engine.SceneComponent|GetRelativeLocation (Variables|Default|GetL1_LeftDoor))) false)
        (Transformation|SetRelativeLocation (+ (Variables|/Script/Engine.SceneComponent|GetRelativeLocation (Variables|Default|GetL1_RightDoor)) _rightspeed) false))
      (:Finished
        (Variables|Default|SetOpening false)))))

(event Input|KeyboardEvents|E
  (:Pressed
    (if (Variables|Default|GetInRange)
      (bind _hasitem (Class|InventoryInterface|CheckInventory(Message) (stale OnComponentBeginOverlap(L1_Collider) OtherActor) "K1"))
      (if _hasitem
        (Variables|Default|SetOpening true)
        (bind _outactors (Actor|GetAllActorsOfClass "/Game/MacabreAssets/Blueprints/FlashlightHUD.FlashlightHUD_C"))
        (Class|HUDInterface|ClearCurrentMessage(Message) (Utilities|Array|Get(acopy) _outactors))
        (Variables|Default|SetIsOpen true)
        (Class|InventoryInterface|RemoveInventory(Message) (Game|GetPlayerCharacter 0) "K1")))))

(fn ConstructionScript)