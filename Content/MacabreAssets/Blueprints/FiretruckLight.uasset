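; Firetruck light Blueprint that alternates two groups of three lights to produce a flashing effect.
; Tick counts down a flicker timer, then switches on CurrentLight to turn one group off and the other to full intensity.
; Each switch toggles the state and resets the timer to a short fixed interval.
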(event EventTick
  (params (DeltaSeconds :type Float%20%28single-precision%29))
  (bind _output_get (Variables|Default|SetFlickerTime (- (Variables|Default|GetFlickerTime) DeltaSeconds)))
  (if (<= _output_get 0.0)
    (switch int (Variables|Default|GetCurrentLight)
      (:0
        (Rendering|Components|Light|SetIntensity 0.0)
        (Rendering|Components|Light|SetIntensity 0.0)
        (Rendering|Components|Light|SetIntensity 0.0)
        (Rendering|Components|Light|SetIntensity 1785.0)
        (Rendering|Components|Light|SetIntensity 1785.0)
        (Rendering|Components|Light|SetIntensity 1785.0)
        (Variables|Default|SetCurrentLight 1))
      (:1
        (Rendering|Components|Light|SetIntensity 1785.0)
        (Rendering|Components|Light|SetIntensity 1785.0)
        (Rendering|Components|Light|SetIntensity 1785.0)
        (Rendering|Components|Light|SetIntensity 0.0)
        (Rendering|Components|Light|SetIntensity 0.0)
        (Rendering|Components|Light|SetIntensity 0.0)
        (Variables|Default|SetCurrentLight 0)))
    (Variables|Default|SetFlickerTime 0.125)))

(fn ConstructionScript)