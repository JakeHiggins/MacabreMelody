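; Donny dialog trigger that plays a sequence of voice lines when the player presses the interact input inside its box.
; The box starts without collision until SwitchDialogTarget enables it; overlap enables input and shows a talk prompt on the FlashlightHUD.
; Each press plays the next DialogElements sound attached to the box.
; After the last line, the box disables collision and clears the prompt.
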(event OnComponentEndOverlap(Box)
  (params (OtherActor :type Actor%20Object%20Reference) (OtherComp :type Primitive%20Component%20Object%20Reference) (OtherBodyIndex :type Integer))
  (Variables|Default|SetInRange false)
  (bind _outactors (Actor|GetAllActorsOfClass "/Game/MacabreAssets/Blueprints/FlashlightHUD.FlashlightHUD_C"))
  (Class|HUDInterface|ClearCurrentMessage(Message) (Utilities|Array|Get(acopy) _outactors)))

(event OnComponentBeginOverlap(Box)
  (params (OtherActor :type Actor%20Object%20Reference) (OtherComp :type Primitive%20Component%20Object%20Reference) (OtherBodyIndex :type Integer) (bFromSweep :type Boolean) (SweepResult :type Hit%20Result%20Structure%20%28by%20ref%29))
  (Variables|Default|SetInRange true)
  (Input|EnableInput (Game|GetPlayerController 0))
  (if (< (Variables|Default|GetCurrentDialog) (Utilities|Array|Length (Variables|Default|GetDialogElements)))
    (bind _outactors (Actor|GetAllActorsOfClass "/Game/MacabreAssets/Blueprints/FlashlightHUD.FlashlightHUD_C"))
    (Default|DisplayMessage (Utilities|Array|Get(acopy) _outactors) "Press 'E' or (X) to talk to Donny")))

(event EventSwitchDialogTarget
  (Collision|SetCollisionEnabled "QueryAndPhysics"))

(event Input|ActionEvents|InputActionEventTrigger
  (:Pressed
    (if (Variables|Default|GetInRange)
      (if (< (Variables|Default|GetCurrentDialog) (Utilities|Array|Length (Variables|Default|GetDialogElements)))
        (Class|GameplayStatics|PlaySoundAttached (Utilities|Array|Get(acopy) (Variables|Default|GetDialogElements) (Variables|Default|GetCurrentDialog)) (Variables|Default|GetBox))
        (Variables|Default|SetCurrentDialog (+ (Variables|Default|GetCurrentDialog) 1))
        (if (not (< (Variables|Default|GetCurrentDialog) (Utilities|Array|Length (Variables|Default|GetDialogElements))))
          (Collision|SetCollisionEnabled "NoCollision")
          (bind _outactors (Actor|GetAllActorsOfClass "/Game/MacabreAssets/Blueprints/FlashlightHUD.FlashlightHUD_C"))
          (Class|HUDInterface|ClearCurrentMessage(Message) (Utilities|Array|Get(acopy) _outactors)))))))

(fn ConstructionScript
  (Collision|SetCollisionEnabled "NoCollision"))