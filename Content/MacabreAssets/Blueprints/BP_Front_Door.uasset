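; BP_Front_Door is a front door that can slam shut and also triggers a one-time audio scare.
; SlamDoor snaps the door's relative transform, plays the slam cue and turns collision on, which the construction script disables initially.
; The first player overlap with the box plays a kid laugh attached to the BP_Stairs_Laugh actor, then a timer plays a locket cue at world origin two seconds later.
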(event OnComponentBeginOverlap(Box)
  (params (OtherActor :type Actor%20Object%20Reference) (OtherComp :type Primitive%20Component%20Object%20Reference) (OtherBodyIndex :type Integer) (bFromSweep :type Boolean) (SweepResult :type Hit%20Result%20Structure%20%28by%20ref%29))
  (if (== OtherActor (Game|Player|GetPlayerPawn 0))
    (if (not (Variables|Default|GetTriggeredLaugh))
      (Variables|Default|SetTriggeredLaugh true)
      (bind _outactors (Actor|GetAllActorsOfClass "/Game/MacabreAssets/Blueprints/AudioTriggers/BP_Stairs_Laugh.BP_Stairs_Laugh_C"))
      (Class|GameplayStatics|PlaySoundAttached "/Game/MacabreAssets/Audio/Kid_Laugh_1_Cue.Kid_Laugh_1_Cue" (Utilities|Array|Get(acopy) (Actor|GetComponentsByClass (Utilities|Array|Get(acopy) _outactors) "/Game/MacabreAssets/Blueprints/AudioTriggers/BP_Laugh_Source.BP_Laugh_Source_C")))
      (Utilities|Time|SetTimerbyFunctionName 0 "PlayBehind" 2.0))))

(event EventSlamDoor
  (Transformation|SetRelativeLocationAndRotation "0, 0,0.000000" "0,180.000000, 0" false)
  (Class|GameplayStatics|PlaySoundAttached "/Game/MacabreAssets/Audio/A_Front_Door_Slam_Cue.A_Front_Door_Slam_Cue" (Variables|Default|GetFrontDoor))
  (Collision|SetCollisionEnabled "QueryAndPhysics"))

(fn ConstructionScript
  (Collision|SetCollisionEnabled "NoCollision"))

(fn PlayBehind
  (Audio|PlaySoundatLocation "/Game/MacabreAssets/Audio/Dialog/Locket/A_Locket_1_Cue.A_Locket_1_Cue" "0, 0, 0"))